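; Test attack gameplay ability that applies GE_TestDamage to a pawn target supplied by the triggering gameplay event.
; Event activation casts the target to Pawn, validates its ability system component, commits, draws a debug arrow from the avatar, then applies the effect.
; CommitAbility is called twice on success, and the ability ends on both success and failure.
; Plain ActivateAbility only prints "Not implemented" and never ends the ability.
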(event Ability|EventActivateAbility
  (Development|PrintString "Not implemented"))

(event Ability|EventActivateAbilityFromEvent
  (params (EventData :type Gameplay%20Event%20Data%20Structure%20%28by%20ref%29))
  (|CallParentFunction EventData)
  (bind _aspawn (Utilities|Casting|CastToPawn (.Target (Utilities|Struct|BreakGameplayEventData EventData)))
    (:then
      (Utilities|IsValid (Ability|GetAbilitySystemComponent _aspawn)
        (:Is%20Valid
          (Variables|Default|SetTargetASC (Ability|GetAbilitySystemComponent _aspawn))
          (bind _returnvalue (Ability|CommitAbility))
          (if _returnvalue
            (Ability|CommitAbility)
            (Rendering|Debug|DrawDebugArrow (Transformation|GetActorLocation (Ability|GetAvatarActorfromActorInfo)) (Transformation|GetActorLocation _aspawn) 15.0 "(R=1.000000,G=0.007402,B=0.000000,A=1.000000)" 3.0 15.0)
            (GameplayEffects|ApplyGameplayEffectToTarget :self (Ability|GetAbilitySystemComponentfromActorInfo) :GameplayEffectClass "/Game/Blueprints/Effects/GE_TestDamage.GE_TestDamage_C" :Target (Variables|Default|GetTargetASC))
            (Ability|EndAbility)
            (else
              (Ability|EndAbility :!label _label))))
        (:Is%20Not%20Valid
          (goto _label))))
    (:CastFailed
      (goto _label))))